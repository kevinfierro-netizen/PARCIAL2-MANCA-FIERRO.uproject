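; BP_Bullet is a projectile from the Super Simple FPS Pack that damages what it overlaps.
; On BeginPlay it switches the ColSphere collision off and immediately back on to query and physics.
; When the sphere begins an overlap with any actor other than the bullet's owner, it applies point damage using its Damage value and the sweep's impact normal as direction.
; The graph does not destroy the bullet after a hit.
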(event `self.ReceiveBeginPlay`
  (bind _colsphere (`self.ColSphere`))
  (`PrimitiveComponent.SetCollisionEnabled` _colsphere "NoCollision")
  (`PrimitiveComponent.SetCollisionEnabled` _colsphere "QueryAndPhysics"))

(event `self.ColSphere.OnComponentBeginOverlap`
  (params (OverlappedComponent :type "PrimitiveComponent Object Reference") (OtherActor :type "Actor Object Reference") (OtherComp :type "PrimitiveComponent Object Reference") (OtherBodyIndex :type Integer) (bFromSweep :type Boolean) (SweepResult :type "HitResult Structure (by ref)"))
  (bind (_bblockinghit _binitialoverlap _time _distance _location _impactpoint _normal _impactnormal _physmat _hitactor) (`GameplayStatics.BreakHitResult` SweepResult))
  (if (!= _hitactor (`self.GetOwner`))
    (`GameplayStatics.ApplyPointDamage` _hitactor (`self.Damage`) _impactnormal SweepResult null self)))

(fn `UserConstructionScript`)