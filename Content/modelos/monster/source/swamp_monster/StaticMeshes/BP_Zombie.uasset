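; BP_Zombie is a jumpscare actor that fires when BP_Player stays in its overlap area for a short delay.
; A cancellable timer triggers the scare: the SwampMonster snaps into place with a 2D scream, a brighter point light, camera shake and a timeline-driven post-process blend.
; Ending overlap clears the timer and, after a scare, runs timelines that move the monster and animate the light, then resets the Screamer flag to re-arm it.
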(event `self.ReceiveActorBeginOverlap`
  (params (OtherActor :type "Actor Object Reference"))
  (if (not (`self.Screamer`))
    (cast `/Game/Super_Simple_FPS_Pack/Character/BP_Player` OtherActor)
    (bind _returnvalue (`KismetSystemLibrary.K2_SetTimerDelegate` (delegate `ActivarEfecto`) 2.0))
    (set `self.TimerEntrada` _returnvalue)))

(event `ActivarEfecto`
  (`|ExecutionSequence`
    (:`then_0`
      (`SceneComponent.K2_SetRelativeLocation` (`self.swamp_monster`) (0.0 30.0 0.0) false false))
    (:`then_1`
      (`GameplayStatics.PlaySound2D` "/Game/Sonido/Zombie_Scream_Sound_Effect.Zombie_Scream_Sound_Effect" 1.0 1.0 0.0 null null))
    (:`then_2`
      (`LightComponent.SetIntensity` (`self.PointLight`) 40.0))
    (:`then_3`
      (`PlayerController.ClientStartCameraShake` :`self` (`GameplayStatics.GetPlayerController` 0) :`Shake` "/Game/SHAKE/BP_Scream.BP_Scream_C"))
    (:`then_4`
      (bind (_direction _newtrack_0) (`Timeline|PostProcessTimeLine` :!via `PlayFromStart`)
        (:`Update`
          (set `PostProcessComponent.BlendWeight` _newtrack_0 (`self.PostProcess`)))))
    (:`then_5`
      (set `self.Screamer` true))))

(event `self.ReceiveActorEndOverlap`
  (params (OtherActor :type "Actor Object Reference"))
  (`KismetSystemLibrary.K2_ClearAndInvalidateTimerHandle` (`self.TimerEntrada`))
  (if (`self.Screamer`)
    (`|ExecutionSequence`
      (:`then_0`
        (bind (_direction _newtrack_0) (`Timeline|RetiradaManoTimeline` :!via `PlayFromStart`)
          (:`Update`
            (`SceneComponent.K2_SetRelativeLocation` (`self.swamp_monster`) (`KismetMathLibrary.VLerp` (0.0 -2281.724686 0.0) (0.0 30.0 0.0) _newtrack_0) false false))
          (:`Finished`
            (set `self.Screamer` false))))
      (:`then_1`
        (bind (_direction_2 _newtrack_0_2) (`Timeline|RetiradaLuzTimeline` :!via `PlayFromStart`)
          (:`Update`
            (`LightComponent.SetIntensity` (`self.PointLight`) (`KismetMathLibrary.Lerp` 0.0 40.0 _newtrack_0_2))))))))

(fn `UserConstructionScript`)